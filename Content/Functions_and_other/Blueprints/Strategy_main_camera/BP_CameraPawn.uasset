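; Strategy camera pawn that glides to the actor under the cursor on a quick click.
; A short delay after press separates holds from taps: a held key sets a flag, cleared on release, while a tap runs a visibility trace under the cursor.
; On a hit, a timeline lerps the pawn from its current location toward that actor.
; The construction script copies the spring arm length into a variable.
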(event Custom|CustomEvent_0
  (params (Hit%20Actor :type Actor%20Object%20Reference))
  (bind _animdrive (Timeline|Focus_Timeline PlayFromStart)
    (:Update
      (Transformation|SetActorLocation (Math|Vector|Lerp(Vector) (Transformation|GetActorLocation) (Transformation|GetActorLocation Hit%20Actor) _animdrive) false false))))

(event Input|ActionEvents|InputActionClick
  (params (Key :type Key%20Structure :default "None"))
  (:Pressed
    (Utilities|FlowControl|Delay 0.2)
    (CallFunction|NewFunction0 Key))
  (:Released
    (Variables|Default|SetNewVar_0 false)))

(fn ConstructionScript
  (LocalVariables|SetNewLocalVar_0 (Variables|/Script/Engine.SpringArmComponent|GetTargetArmLength (Variables|Default|GetSpringArm))))

(fn CheckifClickHitAcrtor
  (bind _returnvalue (Game|GetPlayerController 0))
  (bind _hitresult (Game|Player|GetHitResultUnderCursorbyChannel _returnvalue "TraceTypeQuery1" true))
  (bind (_bblockinghit _binitialoverlap _time _distance _location _impactpoint _normal _impactnormal _physmat _hitactor) (Collision|BreakHitResult _hitresult))
  (return _bblockinghit _hitactor))

(fn NewFunction0
  (params (Key :type Key%20Structure :default "None"))
  (bind (_bblockinghit _hitactor) (CallFunction|CheckifClickHitAcrtor))
  (bind _returnvalue (Game|GetPlayerController 0))
  (bind _returnvalue_2 (Game|Player|IsInputKeyDown _returnvalue Key))
  (if _returnvalue_2
    (Variables|Default|SetNewVar_0 _returnvalue_2)
    (elif _bblockinghit
      (bind _output_get (Variables|Default|SetHit%20Actor _hitactor))
      (CallFunction|CustomEvent0 _output_get))))